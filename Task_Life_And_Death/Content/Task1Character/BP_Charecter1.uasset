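; BP_Charecter1 is a player-controlled character that moves, shoots and recolors the hex grid tiles it touches.
; Input axes drive forward movement along actor facing, plus sideways and vertical movement along world axes.
; Left mouse spawns a bullet at the Arrow's transform, and B spawns BP_Object_1 there.
; Box overlaps give BP_HexGrid meshes a red dynamic material tinted by Color, then a green one on exit.
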(event OnComponentBeginOverlap(Box)
  (params (OverlappedComponent :type Primitive%20Component%20Object%20Reference) (OtherActor :type Actor%20Object%20Reference) (OtherComp :type Primitive%20Component%20Object%20Reference) (OtherBodyIndex :type Integer) (bFromSweep :type Boolean) (SweepResult :type Hit%20Result%20Structure%20%28by%20ref%29))
  ;[1 1 1] Ground Color Change
  (bind _asbp_hex_grid (Utilities|Casting|CastToBP_HexGrid OtherActor))
  (bind _returnvalue (Rendering|Material|CreateDynamicMaterialInstance (Variables|/Game/ThirdPerson/Blueprints/BP_HexGrid.BP_HexGrid_C|GetStaticMesh _asbp_hex_grid) 0 "/Game/ThirdPerson/Blueprints/red.red" "None" :!class /Script/Engine.PrimitiveComponent))
  (Rendering|Material|SetVectorParameterValue _returnvalue "color2" (Variables|Default|GetColor) :!class /Script/Engine.MaterialInstanceDynamic))

(event OnComponentEndOverlap(Box)
  (params (OverlappedComponent :type Primitive%20Component%20Object%20Reference) (OtherActor :type Actor%20Object%20Reference) (OtherComp :type Primitive%20Component%20Object%20Reference) (OtherBodyIndex :type Integer))
  ;[1 1 1] Ground Color Change
  (bind _asbp_hex_grid (Utilities|Casting|CastToBP_HexGrid OtherActor))
  (Rendering|Material|CreateDynamicMaterialInstance (Variables|/Game/ThirdPerson/Blueprints/BP_HexGrid.BP_HexGrid_C|GetStaticMesh _asbp_hex_grid) 0 "/Game/ThirdPerson/Blueprints/green.green" "None" :!class /Script/Engine.PrimitiveComponent))

(event Input|AxisEvents|InputAxisMoveRight/Left
  (params (AxisValue :type Float%20%28single-precision%29))
  ;[1 1 1] Movement
  (Pawn|Input|AddMovementInput (Class|KismetMathLibrary|VectorRight) AxisValue false))

(event Input|AxisEvents|InputAxisMoveForward/Backward
  (params (AxisValue :type Float%20%28single-precision%29))
  ;[1 1 1] Movement
  (Pawn|Input|AddMovementInput (Transformation|GetActorForwardVector) AxisValue false))

(event Input|AxisEvents|InputAxisMoveUp
  (params (AxisValue :type Float%20%28single-precision%29))
  ;[1 1 1] Movement
  (Pawn|Input|AddMovementInput "0.000000,0.000000,1.000000" AxisValue false))

(event Input|KeyboardEvents|B
  (params (Key :type Key%20Structure :default "None"))
  (:Pressed
    (Game|SpawnActorfromClass "/Game/ThirdPerson/Blueprints/BP_Object_1.BP_Object_1_C" (Transformation|GetWorldTransform (Variables|Default|GetArrow)) "Undefined" "OverrideRootScale" 0 0)
    (Collision|IgnoreActorwhenMoving (Variables|Default|GetBox) 0 true)))

(event Input|MouseEvents|LeftMouseButton
  (params (Key :type Key%20Structure :default "None"))
  ;[1 1 1] Bullet
  (:Pressed
    (Game|SpawnActorfromClass "/Game/Task1Character/Bullet/BP_BulletBase_Child.BP_BulletBase_Child_C" (Transformation|GetWorldTransform (Variables|Default|GetArrow)) "Undefined" "MultiplyWithRoot" self 1e+03 0.0 0)
    (Collision|IgnoreActorwhenMoving (Variables|Default|GetBox) 0 true)))

(fn ConstructionScript)